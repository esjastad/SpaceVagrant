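; BP_PlayerCharacter is the player character Blueprint, providing basic directional movement.
; The MoveForward/Backward and MoveLeft/Right axis inputs feed AddMovementInput along the capsule component's forward and right vectors, so movement is relative to the capsule's facing.
; BeginPlay, overlap and Tick are disabled placeholders, and the construction script only calls its parent.
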(event `InputAxis|MoveForward/Backward`
  (params (AxisValue :type "Float (single-precision)"))
  ;[1 1 1] Movement
  (`self.AddMovementInput` (`SceneComponent.GetForwardVector` (`self.CapsuleComponent`)) AxisValue))

(event `InputAxis|MoveLeft/Right`
  (params (AxisValue :type "Float (single-precision)"))
  ;[1 1 1] Movement
  (`self.AddMovementInput` (`SceneComponent.GetRightVector` (`self.CapsuleComponent`)) AxisValue))

(fn `UserConstructionScript`
  (`parent.UserConstructionScript`))