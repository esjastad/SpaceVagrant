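; Trace weapon Blueprint that extends its parent's firing with ammo tracking and a single attachment slot.
; Install stores the attachment properties and marks the slot filled, which GetAttachment reports alongside those properties.
; Fire runs the parent logic, then decrements the loaded ammo without checking for empty.
; Reload moves rounds from the reserve into the clip, capped by free space and remaining ammo, and GetAmmo exposes the counts.
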(event `/Game/Inventory/Attachments/BPI_Install.Install`
  (params (AttachmentProps :type "/Game/Inventory/Attachments/STRUCT_Attachment_Properties Structure"))
  (set `self.AttachmentProps` AttachmentProps)
  (set `self.AttachmentInstalled` true))

(event `/Game/Characters/Assets/Weapons/BPI_WeaponParent.Fire`
  ;[1 1 1] Ammo management
  (`parent.Fire`)
  (`/Engine/EditorBlueprintResources/StandardMacros.DecrementInt` (`self.AmmoLoaded`)))

(event `/Game/Characters/Assets/Weapons/BPI_Ammo.Reload`
  ;[1 1 1] Ammo management
  (if (> (`self.AmmoRemain`) 0)
    (`self.ReloadMath`)))

(fn `Get_Ammo`
  (returns (AmmoLoaded :type Integer) (AmmoRemain :type Integer) (ClipSize :type Integer))
  (return (`self.AmmoLoaded`) (`self.AmmoRemain`) (`self.ClipSize`)))

(fn `GetAttachment`
  (returns (Empty :type Boolean) (AttachmentProps :type "/Game/Inventory/Attachments/STRUCT_Attachment_Properties Structure"))
  (return (not (`self.AttachmentInstalled`)) (`self.AttachmentProps`)))

(fn `ReloadMath`
  (locals (reloadAmount :type Integer :default 0))
  (bind _output_get (set `local.reloadAmount` (`KismetMathLibrary.Min` (`self.AmmoRemain`) (- (`self.ClipSize`) (`self.AmmoLoaded`)))))
  (set `self.AmmoRemain` (- (`self.AmmoRemain`) _output_get))
  (set `self.AmmoLoaded` (+ (`self.AmmoLoaded`) (`local.reloadAmount`))))

(fn `UserConstructionScript`
  (`parent.UserConstructionScript`))