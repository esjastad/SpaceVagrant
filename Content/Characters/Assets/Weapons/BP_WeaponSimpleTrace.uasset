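; BP_WeaponSimpleTrace is a weapon Blueprint whose Fire event shoots along the owning character's camera aim.
; Fire runs a long Visibility line trace from the camera, whose result is unused, then calls FireWeapon.
; FireWeapon spawns a BP_TracerRound at the PointLight's location facing camera forward, and activates the muzzle-flash particles.
; A timeline drives the PointLight's intensity to animate the flash.
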(event `/Game/Characters/Assets/Weapons/BPI_WeaponParent.Fire`
  (bind _camera (`/Game/Characters/MC/MC.Camera` (`self.AimNShootCharRef`)))
  (bind _returnvalue (`SceneComponent.K2_GetComponentLocation` _camera))
  ;[1 1 1] Attempt to Fire weapon
  (`|ExecutionSequence`
    (:`then_0`
      (`KismetSystemLibrary.LineTraceSingle` :`Start` _returnvalue :`End` (+ _returnvalue (* (`SceneComponent.GetForwardVector` _camera) 50000)) :`TraceChannel` "TraceTypeQuery1" :`DrawTime` 1.0))
    (:`then_1`
      (`self.FireWeapon`))))

(event `self.FireWeapon`
  ;[1 1 1] Spawn Bullets
  (`|SpawnActorFromClass` "/Game/ParticleSystems/BP_TracerRound.BP_TracerRound_C" (`KismetMathLibrary.MakeTransform` (`SceneComponent.K2_GetComponentLocation` (`self.PointLight`)) (`KismetMathLibrary.MakeRotFromX` (`SceneComponent.GetForwardVector` (`/Game/Characters/MC/MC.Camera` (`self.AimNShootCharRef`))))) "Undefined" "OverrideRootScale" null null)
  ;[1 1 1] MuzzleFlash
  (`ActorComponent.Activate` (`self.ParticleSystem`) true)
  (bind (_direction _value) (`Timeline|Timeline_0` :!via `PlayFromStart`)
    (:`Update`
      (`LightComponent.SetIntensity` (`self.PointLight`) (* _value 5000.0)))))

(fn `UserConstructionScript`
  (`parent.UserConstructionScript`))