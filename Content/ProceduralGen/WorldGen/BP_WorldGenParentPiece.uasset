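; Parent actor for procedural world generation pieces that snap together at mesh sockets on SimpleCollision.
; On Initialize, a non-start piece picks a socket from the seeded stream and moves and rotates itself to connect there.
; It packages open socket transforms with its piece type and enqueues them on its owner.
; Overlapping pieces destroy themselves; others enable complex collision, and simple collision is removed shortly after.
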(event `/Game/ProceduralGen/WorldGen/BPI_WorldGenPiece.Initialize`
  (params (SEEDGen :type "RandomStream Structure") (`IsStartingPiece?` :type Boolean))
  (set `self.SEEDGen` SEEDGen)
  (set `self.IsStartLocation?` `IsStartingPiece?`)
  (`|ExecutionSequence`
    (:`then_0`
      (`self.PackageEnqueueData`))
    (:`then_1`
      (if (> (`KismetArrayLibrary.Array_Length` (`PrimitiveComponent.GetOverlappingActors` (`self.SimpleCollision`) null)) 0)
        (`self.K2_DestroyActor`)
        (else
          (`PrimitiveComponent.SetCollisionEnabled` (`self.ComplexCollision`) "QueryAndPhysics"))))
    (:`then_2`
      (message `/Game/ProceduralGen/WorldGen/BPI_WorldGenManager.Enqueue` (`self.GetOwner`) (`self.EnqueueData`)))
    (:`then_3`
      (`KismetSystemLibrary.Delay` 0.1)
      (`ActorComponent.K2_DestroyComponent` (`self.SimpleCollision`)))))

(fn `AdjustLocation`
  (params (ConnectingSocketNames :type "Array of Name") (IndexToIgnore :type Integer))
  (locals (ZAngleDeg :type "Float (double-precision)" :default 0.0) (SocketRelativeLoc :type "Vector Structure" :default (0.0 0.0 0.0)))
  (bind (_returnvalue_roll _returnvalue_pitch _returnvalue_yaw) (`KismetMathLibrary.BreakRotator` (`self.K2_GetActorRotation`)))
  (bind _returnvalue (`SceneComponent.GetSocketTransform` (`self.SimpleCollision`) (`|GetArrayItem` ConnectingSocketNames IndexToIgnore) "RTS_Component"))
  (set `local.SocketRelativeLoc` (.location _returnvalue))
  (set `local.ZAngleDeg` (- (+ _returnvalue_yaw 180.0) (.yaw (.rotation _returnvalue))))
  (`self.K2_AddActorWorldOffset` (* (`KismetMathLibrary.RotateAngleAxis` (`local.SocketRelativeLoc`) (`local.ZAngleDeg`) (0.0 0.0 1.0)) (-1.0 -1.0 -1.0)))
  (`self.K2_SetActorRotation` (`KismetMathLibrary.MakeRotator` 0.0 0.0 (`local.ZAngleDeg`))))

(fn `GetARandomIndex`
  (params (`Target Array` :type "Array of Name"))
  (returns (Index :type Integer))
  (return (`KismetMathLibrary.RandomIntegerInRangeFromStream` 0 (- (`KismetArrayLibrary.Array_Length` `Target Array`) 1) (`self.SEEDGen`))))

(fn `PackageEnqueueData`
  (locals (Temp :type "Array of Transform Structure") (IndexToIgnore :type Integer))
  (bind _returnvalue (`self.GetTransform`))
  (bind _returnvalue_2 (`self.GetTransform`))
  (bind _returnvalue_3 (`SceneComponent.GetAllSocketNames` (`self.SimpleCollision`)))
  ;[1 1 1] Does Piece = Platformer
  (if (== (`self.PieceType`) 8)
    (`KismetSystemLibrary.PrintString` "Platformer Not implemented yet")
    (elif (`self.IsStartLocation?`)
      (`KismetArrayLibrary.Array_Clear` (`local.Temp`))
      (for _array_element (`SceneComponent.GetAllSocketNames` (`self.SimpleCollision`))
        (bind _returnvalue_4 (`SceneComponent.GetSocketTransform` (`self.SimpleCollision`) _array_element "RTS_Component"))
        (`KismetArrayLibrary.Array_Add` (`local.Temp`) (`KismetMathLibrary.MakeTransform` (+ (.location _returnvalue) (`KismetMathLibrary.RotateAngleAxis` (.location _returnvalue_4) (.yaw (.rotation _returnvalue)) (0.0 0.0 1.0))) (`KismetMathLibrary.MakeRotator` 0.0 0.0 (+ (.yaw (.rotation _returnvalue_4)) (.yaw (.rotation _returnvalue)))))))
      (set `self.EnqueueData` (make `/Game/ProceduralGen/WorldGen/STRUCT_WorldGenEnqueueData` (`self.PieceType`) (`local.Temp`)))
      (else
        (`KismetArrayLibrary.Array_Clear` (`local.Temp`))
        (if (`KismetArrayLibrary.Array_IsValidIndex` _returnvalue_3)
          (set `local.IndexToIgnore` (`self.GetARandomIndex` _returnvalue_3))
          (`self.AdjustLocation` _returnvalue_3 (`local.IndexToIgnore`))
          (for (_array_element_2 _array_index) _returnvalue_3
            (if (not (== _array_index (`local.IndexToIgnore`)))
              (bind _returnvalue_5 (`SceneComponent.GetSocketTransform` (`self.SimpleCollision`) _array_element_2 "RTS_Component"))
              ;[1 1 1] Need to check and break up socket names for additional piece spawning
              (`KismetArrayLibrary.Array_Add` (`local.Temp`) (`KismetMathLibrary.MakeTransform` (+ (.location _returnvalue_2) (`KismetMathLibrary.RotateAngleAxis` (.location _returnvalue_5) (.yaw (.rotation _returnvalue_2)) (0.0 0.0 1.0))) (`KismetMathLibrary.MakeRotator` 0.0 0.0 (+ (.yaw (.rotation _returnvalue_5)) (.yaw (.rotation _returnvalue_2))))))))
          (set `self.EnqueueData` (make `/Game/ProceduralGen/WorldGen/STRUCT_WorldGenEnqueueData` (`self.PieceType`) (`local.Temp`)))
          (else
            (`KismetSystemLibrary.PrintString` "Error, Mesh has no valid connection sockets")
            (`self.K2_DestroyActor`)))))))

(fn `UserConstructionScript`)