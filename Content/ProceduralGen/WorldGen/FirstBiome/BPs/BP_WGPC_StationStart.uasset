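; BP_WGPC_StationStart is a station start Blueprint in the first biome's procedural world generation that restores the player character's physical state.
; On BeginPlay it calls the parent, waits briefly, then re-enables capsule query-and-physics collision and mesh query-only collision, and sets gravity scale back to normal on player 0.
; The construction script only calls its parent, and overlap and Tick are disabled.
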(event `self.ReceiveBeginPlay`
  (bind _returnvalue (`GameplayStatics.GetPlayerCharacter` 0))
  (`parent.ReceiveBeginPlay`)
  (`KismetSystemLibrary.Delay` 0.1)
  (`PrimitiveComponent.SetCollisionEnabled` (`Character.CapsuleComponent` _returnvalue) "QueryAndPhysics")
  (`PrimitiveComponent.SetCollisionEnabled` (`Character.Mesh` _returnvalue) "QueryOnly")
  (set `CharacterMovementComponent.GravityScale` 1.0 (`Character.CharacterMovement` _returnvalue)))

(fn `UserConstructionScript`
  (`parent.UserConstructionScript`))