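; World generator manager actor that procedurally builds a level from randomly chosen piece classes, beginning with a start piece on BeginPlay.
; Connection data received through Enqueue is processed one entry per Tick, spawning pieces at its transforms, gated by a world bounds check.
; A comma-separated neighbor map picks each piece type, with random selection drawn from a seeded stream.
; Tick stops at the size limit or when the queue stays empty.
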(event `/Game/ProceduralGen/WorldGen/BPI_WorldGenManager.Enqueue`
  (params (DataToEnqueue :type "/Game/ProceduralGen/WorldGen/STRUCT_WorldGenEnqueueData Structure"))
  ;[1 1 1] Enqueue Data Message
  (`KismetArrayLibrary.Array_Add` (`self.EnqueueData`) DataToEnqueue))

(event `self.ReceiveBeginPlay`
  (bind _output_classreferences (break `/Game/ProceduralGen/WorldGen/STRUCT_WorldGenPieceClass` (`|GetArrayItem` (`self.PrototypeClasses`) 1)))
  (`|ExecutionSequence`
    (:`then_0`
      ;[1 1 1] Set spawn control variables to their default state
      (`self.ClearSpawnControls`))
    (:`then_1`
      ;[1 1 1] Spawn the level start piece
      (bind _returnvalue (`|SpawnActorFromClass` (`|GetArrayItem` _output_classreferences (`KismetMathLibrary.RandomIntegerInRangeFromStream` 0 (- (`KismetArrayLibrary.Array_Length` _output_classreferences) 1) (`self.SeedGen`))) (`self.NextSpawnXForm`) "Undefined" "OverrideRootScale" self null))
      (message `/Game/ProceduralGen/WorldGen/BPI_WorldGenPiece.Initialize` _returnvalue (`self.SeedGen`) true))
    (:`then_2`
      ;[1 1 1] Enable Actor Tick
      (`self.SetActorTickEnabled` true))))

(event `self.ReceiveTick`
  (params (DeltaSeconds :type "Float (single-precision)"))
  (bind _output_piecetype (break `/Game/ProceduralGen/WorldGen/STRUCT_WorldGenEnqueueData` (`|GetArrayItem` (`self.EnqueueData`))))
  (bind (_output_piecetype_2 _output_connectingxforms) (break `/Game/ProceduralGen/WorldGen/STRUCT_WorldGenEnqueueData` (`|GetArrayItem` (`self.EnqueueData`))))
  ;[1 1 1] Check if we hit our world gen size limit
  (if (> (`self.GenSize`) (`self.SpawnIteration`))
    ;[1 1 1] Check if there is valid queued data
    (if (`KismetArrayLibrary.Array_IsValidIndex` (`self.EnqueueData`))
      ;[1 1 1] Loop through the queued data and spawn an appropriate connecting piece
      (for _array_element _output_connectingxforms
        (bind (_nextpieceindex _valid_) (`self.GetValidNeighborType` (`KismetMathLibrary.Conv_ByteToInt` _output_piecetype)))
        (if _valid_
          (set `self.NextClassIndex` _nextpieceindex)
          (if (`self.ExceedsBoundsCheck` _array_element)
            (bind _returnvalue (`|SpawnActorFromClass` (`self.GetAWorldPieceClassToSpawn`) _array_element "Undefined" "OverrideRootScale" self null))
            (message `/Game/ProceduralGen/WorldGen/BPI_WorldGenPiece.Initialize` _returnvalue (`self.SeedGen`) false))))
      ;[1 1 1] Remove the completed queue data
      (`KismetArrayLibrary.Array_Remove` (`self.EnqueueData`))
      (`/Engine/EditorBlueprintResources/StandardMacros.IncrementInt` (`self.SpawnIteration`))
      (else
        ;[1 1 1] If no valid data is remaining in the queue or we hit our gen limit, turn off event tick in this actor
        (`self.SetActorTickEnabled` false)
        (`KismetSystemLibrary.Delay` 0.25)
        (if (`KismetArrayLibrary.Array_IsValidIndex` (`self.EnqueueData`))
          (`self.SetActorTickEnabled` true)
          (else
            (`KismetSystemLibrary.PrintString` "Index 0 invalid")
            (`self.SetActorTickEnabled` false :!label _label)))))
    (else
      (`KismetSystemLibrary.PrintString` "Gen size hit!" true true (struct :`G` 0.66 :`B` 1.0 :`A` 1.0) 22.0)
      (goto _label))))

(fn `ClearSpawnControls`
  (`KismetArrayLibrary.Array_Clear` (`self.EnqueueData`))
  (set `self.NextSpawnXForm` (`KismetMathLibrary.MakeTransform` (0.0 0.0 0.0)))
  (set `self.SpawnIteration` 0))

(fn `ExceedsBoundsCheck`
  (params (Tranform :type "Transform Structure"))
  (returns (`Valid?` :type Boolean))
  (bind (_worldbounds_x _worldbounds_y) (`KismetMathLibrary.BreakVector` (`self.WorldBounds`)))
  (bind (_worldbounds_x_2 _worldbounds_y_2) (`KismetMathLibrary.BreakVector` (`self.WorldBounds`)))
  (return (or (< (.x (.location Tranform)) _worldbounds_x_2) (< (.y (.location Tranform)) _worldbounds_y_2) (> (.x (.location Tranform)) (* _worldbounds_x -1.0)) (> (.y (.location Tranform)) (* _worldbounds_y -1.0)))))

(fn `GetAWorldPieceClassToSpawn`
  (returns (Output :type "Actor Class Reference"))
  (bind _output_classreferences (break `/Game/ProceduralGen/WorldGen/STRUCT_WorldGenPieceClass` (`|GetArrayItem` (`self.PrototypeClasses`) (`self.NextClassIndex`))))
  (return (`|GetArrayItem` _output_classreferences (`KismetMathLibrary.RandomIntegerInRangeFromStream` 0 (- (`KismetArrayLibrary.Array_Length` _output_classreferences) 1) (`self.SeedGen`)))))

(fn `GetValidNeighborType`
  (params (PieceTypeEnum :type Integer))
  (returns (NextPieceIndex :type Integer) (`Valid?` :type Boolean))
  (bind (_value _returnvalue) (`BlueprintMapLibrary.Map_Find` (`self.NeighborMapping`) (cast `/Game/ProceduralGen/WorldGen/ENUM_WorldGenPieceType` (`KismetMathLibrary.Conv_IntToByte` PieceTypeEnum))))
  (bind _returnvalue_2 (`KismetStringLibrary.ParseIntoArray` _value ","))
  ;[1 1 1] Find valid mapping string
  (if _returnvalue
    ;[1 1 1] Parse the string delimiting by a ',' and check if there are any valid entries
    (if (`KismetArrayLibrary.Array_IsValidIndex` _returnvalue_2)
      (return (`KismetStringLibrary.Conv_StringToInt` (`|GetArrayItem` _returnvalue_2 (`KismetMathLibrary.RandomIntegerInRangeFromStream` 0 (- (`KismetArrayLibrary.Array_Length` _returnvalue_2) 1) (`self.SeedGen`)))) true)
      (else
        _)))
  (return -1 false))

(fn `UserConstructionScript`)