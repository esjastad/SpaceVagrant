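; BP_Inventory is an inventory Blueprint that tracks resource amounts in the ResourcePool array of resource and amount slots.
; AddResource searches the pool for a slot with the same resource class, adds the incoming amount to it and stops.
; A resource class with no existing slot is not added.
; The EventGraph holds only a disconnected, incomplete copy of the same loop, which never runs.
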(fn `AddResource`
  (params (ResuorceSlot :type "/Game/Inventory/STRUCT_ResourceSlot Structure"))
  (bind (_resource _amount) (break `/Game/Inventory/STRUCT_ResourceSlot` ResuorceSlot))
  (for (_array_element _array_index) (`self.ResourcePool`)
    (if (== (`.class_18_C382EAE040AF0FA6F853ACA100CAB975` (break `/Game/Inventory/STRUCT_Resource` (break `/Game/Inventory/STRUCT_ResourceSlot` _array_element))) (`.class_18_C382EAE040AF0FA6F853ACA100CAB975` (break `/Game/Inventory/STRUCT_Resource` _resource)))
      (bind _output_resource (break `/Game/Inventory/STRUCT_ResourceSlot` (`|GetArrayItem` (`self.ResourcePool`) _array_index)))
      (`KismetArrayLibrary.Array_Set` (`self.ResourcePool`) _array_index (make `/Game/Inventory/STRUCT_ResourceSlot` _output_resource (+ (`.Amount_5_D9E696AA4B12ED80908E85B6EABB7C80` (break `/Game/Inventory/STRUCT_ResourceSlot` _array_element)) _amount)))
      (break))))